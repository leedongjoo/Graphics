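; RoadMovement_BP is a road actor meant to slide its static mesh along world Y, but the movement is currently not triggered.
; BeginPlay only enables input for the first player controller.
; An unconnected chain stores the mesh's start position, offsets its Y with a timeline track, then increments and prints RoadMovementCount on finish.
; A Korean note marks that movement is to be switched to a UI press.
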(event EventBeginPlay
  (Input|EnableInput (Game|GetPlayerController 0)))

(event Input|KeyboardEvents|SpaceBar
  (params (Key :type Key%20Structure :default "None")))

(fn ConstructionScript)