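; PlaneManager is an actor that serves as the player's view target and manages a plane with an actor spawner.
; BeginPlay enables input and switches the view to itself.
; The Spawn event calls PineTreeSpawner, which spawns one actor at Arrow1's location and ignores SpawnNum.
; Timeline logic to raise and roll the plane in up to three guarded steps each is present but disconnected, so it never runs.
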(event Custom|Spawn
  ;[1 1 1] 스폰
  (CallFunction|PineTreeSpawner (Variables|Default|GetSpawnNum)))

(event EventBeginPlay
  (bind _returnvalue (Game|GetPlayerController 0))
  (Input|EnableInput _returnvalue)
  (Game|Player|SetViewTargetwithBlend _returnvalue self 0.0 "VTBlend_Linear" 0.0 false))

(event Input|KeyboardEvents|SpaceBar
  (params (Key :type Key%20Structure :default "None")))

(event Input|KeyboardEvents|SpaceBar
  (params (Key :type Key%20Structure :default "None"))
  ;[1 1 1] 회전변환
)

(fn ConstructionScript)

(fn PineTreeSpawner
  (params (SpawnNum :type Integer))
  (Game|SpawnActorfromClass "/Game/main/Blueprints/SM_pineTree_C4_Blueprint.SM_pineTree_C4_Blueprint_C" (Math|Transform|MakeTransform (Transformation|GetWorldLocation (Variables|Default|GetArrow1)) "0, 0, 0" "1,1,1") "AlwaysSpawn" 0 0))